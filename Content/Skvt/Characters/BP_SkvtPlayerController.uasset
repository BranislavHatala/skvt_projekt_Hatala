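; Player controller for Skvt characters that handles pawn swapping, camera zoom and crouch toggling through Enhanced Input.
; On BeginPlay it adds the default, swap-pawn and camera-zoom mapping contexts.
; Swap possesses the next BP_SkvtBaseChar in the level's actor list, wrapping around.
; Zoom adjusts the controlled pawn's spring arm length by scroll input, and crouch toggles on the first player's character.
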(event Input|EnhancedActionEvents|EnhancedInputActionIA_Swap
  (params (ActionValue :type Boolean) (ElapsedSeconds :type Float%20%28double-precision%29) (TriggeredSeconds :type Float%20%28double-precision%29) (InputAction :type Input%20Action%20Object%20Reference :default "/Game/Skvt/Characters/Input/Actions/IA_Swap.IA_Swap"))
  (:Triggered
    (bind _outactors (Actor|GetAllActorsOfClass "/Game/Skvt/Characters/BP_SkvtBaseChar.BP_SkvtBaseChar_C"))
    (bind _asbp_skvt_base_char (Utilities|Casting|CastToBP_SkvtBaseChar (Pawn|GetControlledPawn self)))
    (if (Utilities|Array|IsValidIndex _outactors (Math|Integer|%(Integer) (+ (Utilities|Array|FindItem _outactors _asbp_skvt_base_char) 1) (Utilities|Array|Length _outactors)))
      (Pawn|Possess (Utilities|Array|Get(acopy) _outactors (Math|Integer|%(Integer) (+ (Utilities|Array|FindItem _outactors _asbp_skvt_base_char) 1) (Utilities|Array|Length _outactors)))))))

(event Input|EnhancedActionEvents|EnhancedInputActionCameraZoom
  (params (ActionValue :type Float%20%28double-precision%29) (ElapsedSeconds :type Float%20%28double-precision%29) (TriggeredSeconds :type Float%20%28double-precision%29) (InputAction :type Input%20Action%20Object%20Reference :default "/Game/Skvt/Characters/Input/Actions/CameraZoom.CameraZoom"))
  (bind _self self)
  (bind _returnvalue (Pawn|GetControlledPawn _self))
  (bind _returnvalue_2 (Actor|GetComponentbyClass _returnvalue "/Script/Engine.SpringArmComponent"))
  (:Triggered
    (Utilities|IsValid _returnvalue_2
      (:Is%20Valid
        (Variables|/Script/Engine.SpringArmComponent|SetTargetArmLength _returnvalue_2 (+ (Variables|/Script/Engine.SpringArmComponent|GetTargetArmLength _returnvalue_2) (* ActionValue (Variables|Default|GetScrollSpeed))))))))

(event Input|EnhancedActionEvents|EnhancedInputActionCrouchToggle
  (params (ActionValue :type Boolean) (ElapsedSeconds :type Float%20%28double-precision%29) (TriggeredSeconds :type Float%20%28double-precision%29) (InputAction :type Input%20Action%20Object%20Reference :default "/Game/Skvt/Characters/Input/Actions/CrouchToggle.CrouchToggle"))
  (:Started
    (bind _asbp_skvt_base_char (Utilities|Casting|CastToBP_SkvtBaseChar (Game|Player|GetPlayerPawn 0)))
    (Variables|Default|SetAs%20BP%20Skvt%20Base%20Char _asbp_skvt_base_char)
    (if (AI|Components|NavMovement|IsCrouching (Variables|/Script/Engine.Character|GetCharacterMovement _asbp_skvt_base_char))
      (Character|UnCrouch (Variables|Default|GetAs%20BP%20Skvt%20Base%20Char))
      (else
        (Character|Crouch (Variables|Default|GetAs%20BP%20Skvt%20Base%20Char))))))

(event EventBeginPlay
  (bind _self self)
  (bind _returnvalue (PlayerController|LocalPlayerSubsystems|GetEnhancedInputLocalPlayerSubsystem _self))
  (Development|PrintString "Hello")
  (Utilities|IsValid _returnvalue
    (:Is%20Valid
      (Utilities|FlowControl|Sequence
        (:then_0
          (Input|AddMappingContext _returnvalue "/Game/ThirdPerson/Input/IMC_Default.IMC_Default" 0 "(bIgnoreAllPressedKeysUntilRelease=True,bForceImmediately=False)"))
        (:then_1
          (Input|AddMappingContext _returnvalue "/Game/Skvt/Characters/Input/IMC_SwapPawn.IMC_SwapPawn" 0 "(bIgnoreAllPressedKeysUntilRelease=True,bForceImmediately=False)"))
        (:then_2
          (Input|AddMappingContext _returnvalue "/Game/Skvt/Characters/Input/IMC_Camera_zoom.IMC_Camera_zoom" 0 "(bIgnoreAllPressedKeysUntilRelease=True,bForceImmediately=False)"))))))

(fn ConstructionScript)