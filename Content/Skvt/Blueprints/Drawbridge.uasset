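; Drawbridge actor that can be broken once to swing its bridge piece into a new position.
; BreakDown guards against repeat calls with a Broken flag, spawns a short burst of sparks at the point light, then switches the light off.
; A timeline then drives the Scene component's pitch to animate the movement.
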(event EventBeginPlay)

(event Collision|EventActorBeginOverlap
  (params (OtherActor :type Actor%20Object%20Reference)))

(event EventTick
  (params (DeltaSeconds :type Float%20%28single-precision%29)))

(event EventBreakDown
  (if (not (Variables|Default|GetBroken))
    (Variables|Default|SetBroken true)
    (bind _returnvalue (Effects|SpawnEmitteratLocation "/Game/StarterContent/Particles/P_Sparks.P_Sparks" (Transformation|GetWorldLocation (Variables|Default|GetPointLight)) "0, 0, 0" "1.000000,1.000000,1.000000" false))
    (Utilities|FlowControl|Delay 0.2)
    (Components|Activation|Deactivate _returnvalue)
    (Rendering|Components|Light|SetIntensity (Variables|Default|GetPointLight) 0.0)
    (bind _newtrack_0 (Timeline|Timeline PlayFromStart)
      (:Update
        (Transformation|SetRelativeRotation (Variables|Default|GetScene) (Math|Rotator|MakeRotator 0.0 _newtrack_0 0.0) false false)))))

(fn ConstructionScript)